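; BP_FlyingAI is a flying AI actor that bobs vertically between upward and downward movement.
; Each Tick moves it through the movement component by Speed up or down according to IsUp, keeping its current rotation.
; A Clock accumulates delta time and flips IsUp each time it reaches ChangeDirectionValue, then resets.
; The per-frame step is not scaled by delta time, so travel distance depends on frame rate.
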(event EventTick
  (params (DeltaSeconds :type Float%20%28single-precision%29))
  (bind _returnvalue (Transformation|GetActorRotation))
  (bind _charactermovement (Variables|Character|GetCharacterMovement))
  (bind _speed (Variables|Default|GetSpeed))
  (if (Variables|Default|GetIsUp)
    (Class|MovementComponent|MoveUpdatedComponent _charactermovement (Math|Vector|MakeVector 0.0 0.0 _speed) _returnvalue true)
    (else
      (Class|MovementComponent|MoveUpdatedComponent _charactermovement (Math|Vector|MakeVector 0.0 0.0 (* _speed -1.0)) _returnvalue true)))
  (Variables|Default|SetClock (+ DeltaSeconds (Variables|Default|GetClock)))
  (if (>= (Variables|Default|GetClock) (Variables|Default|GetChangeDirectionValue))
    (Variables|Default|SetIsUp (not (Variables|Default|GetIsUp)))
    (Variables|Default|SetClock 0.0)))

(fn ConstructionScript)