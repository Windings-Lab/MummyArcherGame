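; Game mode that assigns teams to mummy characters and places them at team spawn points once the required players have connected.
; Tick waits for the character count to match PlayersNeedToConnect, then after a delay copies each controller's team number to its character.
; It then teleports each character to a free matching BP_MummyPlayerStart, claims it, stores the spawn rotation and latches off.
; A note marks the Tick logic for a C++ rewrite.
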(event EventBeginPlay)

(event EventTick
  (params (DeltaSeconds :type Float%20%28single-precision%29))
  (if (not (Variables|Default|GetLocalStopTick))
    (if (Variables|Default|GetTeamsSetUpDone)
      (bind _outactors (Actor|GetAllActorsOfClass "/Game/GameRules/BP_MummyPlayerStart.BP_MummyPlayerStart_C"))
      (bind _outactors_2 (Actor|GetAllActorsOfClass "/Game/Characters/Blueprints/BP_MummyCharacter.BP_MummyCharacter_C"))
      (for _array_element _outactors_2
        (Variables|/Game/Characters/Blueprints/BP_MummyCharacter.BP_MummyCharacter_C|SetTeamsSetUpDone _array_element true)
        (bind _array_element_2 (Utilities|Array|ForEachLoopwithBreak _outactors :!label _label)
          (:LoopBody
            (if (Default|IsFree _array_element_2)
              (if (== (Default|GetTeamNumber _array_element_2) (Variables|/Game/Characters/Blueprints/BP_MummyCharacter.BP_MummyCharacter_C|GetTeam _array_element))
                (bind _returnvalue (Transformation|SetActorLocationAndRotation _array_element (.location (Transformation|GetActorTransform _array_element_2)) (.rotation (Transformation|GetActorTransform _array_element_2)) false true))
                (Variables|/Game/Characters/Blueprints/BP_MummyCharacter.BP_MummyCharacter_C|SetSpawnRotation _array_element (.rotation (Transformation|GetActorTransform _array_element_2)))
                (Variables|/Script/MummyArcherGame.MummyPlayerStart|SetbIsFree _array_element_2 (not _returnvalue))
                (goto _label Break))))))
      (Variables|Default|SetLocalStopTick true)
      (else
        (bind _outactors_3 (Actor|GetAllActorsOfClass "/Game/Characters/Blueprints/BP_MummyCharacter.BP_MummyCharacter_C"))
        (if (== (Utilities|Array|Length _outactors_3) (Variables|Default|GetPlayersNeedToConnect))
          (Utilities|FlowControl|Delay 2.0)
          (bind _outactors_4 (Actor|GetAllActorsOfClass "/Game/Characters/Blueprints/BP_MummyCharacter.BP_MummyCharacter_C"))
          (for _array_element_3 _outactors_4
            (bind _asbp_mummy_player_controller (Utilities|Casting|CastToBP_MummyPlayerController (Pawn|GetController _array_element_3)))
            (Variables|/Game/Characters/Blueprints/BP_MummyCharacter.BP_MummyCharacter_C|SetTeam _array_element_3 (Variables|/Script/MummyArcherGame.MummyPlayerController|GetTeamNumber _asbp_mummy_player_controller)))
          (Variables|Default|SetTeamsSetUpDone true))))))

(fn ConstructionScript)