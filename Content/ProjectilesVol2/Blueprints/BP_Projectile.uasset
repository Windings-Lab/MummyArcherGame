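; BP_Projectile is a projectile actor that plays a muzzle flash effect on spawn and an impact effect when its sphere hits something.
; The hit effect spawns at a normal-offset point, oriented to zero, the actor's rotation, or the impact normal, chosen by flags.
; On hit it switches off its point light and destroys itself after a configurable delay, with a ten-second lifetime fallback otherwise.
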(event OnComponentHit(Sphere)
  (params (HitComponent :type Primitive%20Component%20Object%20Reference) (OtherActor :type Actor%20Object%20Reference) (OtherComp :type Primitive%20Component%20Object%20Reference) (NormalImpulse :type Vector :default "0, 0, 0") (Hit :type Hit%20Result%20Structure%20%28by%20ref%29))
  (bind (_bblockinghit _binitialoverlap _time _distance _location _impactpoint _normal _impactnormal) (Collision|BreakHitResult Hit))
  (if (Variables|Default|GetUse%20zero%20rotation)
    (Variables|Default|SetRotation "0, 0, 0")
    (elif (Variables|Default|GetUse%20self%20rotation)
      (Variables|Default|SetRotation (Transformation|GetActorRotation))
      (else
        (Variables|Default|SetRotation (Math|Rotator|MakeRotfromX _impactnormal)))))
  (Niagara|SpawnSystematLocation (Variables|Default|GetHit%20effect) (+ _location (* _impactnormal (Variables|Default|GetHit%20offset))) (Variables|Default|GetRotation) (Variables|Default|GetScale))
  (Rendering|Components|Light|SetIntensity (Variables|Default|GetPointLight) 0.0)
  (Utilities|FlowControl|Delay (Variables|Default|GetProjectile%20hit%20destroy%20delay))
  (Actor|DestroyActor))

(event EventBeginPlay
  (Niagara|SpawnSystematLocation (Variables|Default|GetFlash%20effect) (Transformation|GetActorLocation) (Transformation|GetActorRotation) (Variables|Default|GetScale))
  (Utilities|FlowControl|Delay 1e+01)
  (Actor|DestroyActor))

(fn ConstructionScript)